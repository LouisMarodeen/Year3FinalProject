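; Enemy turret that registers with the game mode's alive count and attacks the player with a targeting beam.
; Tick either sweeps the body bone side to side or runs the attack state.
; PawnSensing aims the bone at tagged pawns, traces the Niagara beam endpoint and restarts a one-second timer that reverts to searching.
; After six seconds of targeting, it recolours the beam, directly deducts one health, then cools down.
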(event OnSeePawn(PawnSensing)
  (params (Pawn :type Pawn%20Object%20Reference))
  (bind _poseablemesh (Variables|Default|GetPoseableMesh))
  (if (Actor|ActorHasTag Pawn "TurretTarget")
    (Variables|Default|SetIsBeamActive true)
    (Variables|Default|SetTargetLocation (Transformation|GetActorLocation Pawn))
    (Variables|Default|SetTurretState "NewEnumerator1")
    (bind _returnvalue (Class|PoseableMeshComponent|GetBoneRotationbyName _poseablemesh "bn_body" "WorldSpace"))
    (bind _output_get (Variables|Default|SetRotation (Math|Rotator|MakeRotator (.roll _returnvalue) (- (.pitch (Math|Rotator|FindLookatRotation (Transformation|GetActorLocation) (Variables|Default|GetTargetLocation))) 15.0) (.yaw (Math|Rotator|FindLookatRotation (Transformation|GetActorLocation) (Variables|Default|GetTargetLocation))))))
    (Components|PoseableMesh|SetBoneRotationbyName _poseablemesh "bn_body" _output_get "WorldSpace")
    (Utilities|FlowControl|Sequence
      (:then_0
        (if (not (Variables|Default|GetIsAttacking))
          (Components|Activation|Activate (Variables|Default|GetBeam) false)))
      (:then_1
        (CallFunction|UpdateBeam)
        (Utilities|FlowControl|DelayUntilNextTick)
        (Utilities|Time|ClearandInvalidateTimerbyHandle (Variables|Default|GetResetTurretTimer))
        (bind _returnvalue_2 (Utilities|Time|SetTimerbyEvent (delegate Custom|ResetTurretState) 1.0))
        (Variables|Default|SetResetTurretTimer _returnvalue_2)))))

(event Custom|RotateTurret
  (bind _returnvalue (Utilities|Time|GetWorldDeltaSeconds))
  (bind _returnvalue_2 (* _returnvalue 5e+01))
  (bind _returnvalue_3 (Class|PoseableMeshComponent|GetBoneRotationbyName (Variables|Default|GetPoseableMesh) "bn_body" "ComponentSpace"))
  (Variables|Default|SetTurretRotateRight (or (and (< (.Yaw (Math|Rotator|BreakRotator _returnvalue_3)) 7e+01) (Variables|Default|GetTurretRotateRight)) (and (< (.Yaw (Math|Rotator|BreakRotator _returnvalue_3)) -7e+01) (not (Variables|Default|GetTurretRotateRight)))))
  (Components|PoseableMesh|SetBoneRotationbyName (Variables|Default|GetPoseableMesh) "bn_body" (Math|Rotator|MakeRotator (.Roll (Math|Rotator|BreakRotator _returnvalue_3)) (.Pitch (Math|Rotator|BreakRotator _returnvalue_3)) (Math|Float|SelectFloat (+ (.Yaw (Math|Rotator|BreakRotator _returnvalue_3)) _returnvalue_2) (- (.Yaw (Math|Rotator|BreakRotator _returnvalue_3)) _returnvalue_2) (Variables|Default|GetTurretRotateRight))) "ComponentSpace")
  (Variables|Default|SetTargetingTime 0.0))

(event Custom|AttackTurret
  (if (> (Variables|Default|GetTargetingTime) 6.0)
    (if (not (Variables|Default|GetIsAttacking))
      (Variables|Default|SetIsAttacking true)
      (Niagara|SetNiagaraVariable(LinearColor) (Variables|Default|GetBeam) "User.Color" (Variables|Default|GetTargetColour))
      (Audio|PlaySound2D "/Game/Sounds/SFX/Sci-Fi_Gun_1-1.Sci-Fi_Gun_1-1" 1.0 1.0 0.0 0 0)
      (bind _asbp_first_person_character (Utilities|Casting|CastToBP_FirstPersonCharacter (stale OnSeePawn(PawnSensing) Pawn)))
      (bind _output_get (Variables|Default|SetAs%20BP%20First%20Person%20Character _asbp_first_person_character))
      (bind _output_get_2 (Variables|/Game/FirstPerson/Blueprints/BP_FirstPersonCharacter.BP_FirstPersonCharacter_C|SetCurrentHealth _output_get (Math|Integer|Max(Integer) 0 (- (Variables|/Game/FirstPerson/Blueprints/BP_FirstPersonCharacter.BP_FirstPersonCharacter_C|GetCurrentHealth _output_get) 1))))
      (Default|SetHealth (Variables|/Game/FirstPerson/Blueprints/BP_FirstPersonCharacter.BP_FirstPersonCharacter_C|GetHealthWidget _output_get) _output_get_2)
      (Default|IsCharacterDead _asbp_first_person_character)
      (Utilities|FlowControl|Delay 2.0)
      (Components|Activation|Deactivate (Variables|Default|GetBeam))
      (Utilities|FlowControl|Delay (Variables|Default|GetDelayBetweenAttacks))
      (Niagara|SetNiagaraVariable(LinearColor) (Variables|Default|GetBeam) "User.Color" (Variables|Default|GetAttackColour))
      (Variables|Default|SetTargetingTime 0.0)
      (Variables|Default|SetIsAttacking false))))

(event Custom|ResetTurretState
  (Development|PrintText "Searching")
  (Variables|Default|SetTurretState "NewEnumerator0")
  (Variables|Default|SetTargetingTime 0.0)
  (Variables|Default|SetIsBeamActive false)
  (Components|Activation|Deactivate (Variables|Default|GetBeam)))

(event EventBeginPlay
  (bind _asbp_first_person_game_mode (Utilities|Casting|CastToBP_FirstPersonGameMode (Game|GetGameMode)))
  (Variables|/Game/FirstPerson/Blueprints/BP_FirstPersonGameMode.BP_FirstPersonGameMode_C|SetEnemiesAlive _asbp_first_person_game_mode (+ (Variables|/Game/FirstPerson/Blueprints/BP_FirstPersonGameMode.BP_FirstPersonGameMode_C|GetEnemiesAlive _asbp_first_person_game_mode) 1)))

(event Collision|EventActorBeginOverlap
  (params (OtherActor :type Actor%20Object%20Reference)))

(event EventTick
  (params (DeltaSeconds :type Float%20%28single-precision%29))
  (Variables|Default|SetTargetingTime (+ DeltaSeconds (Variables|Default|GetTargetingTime)))
  (switch Utilities|FlowControl|Switch|SwitchonTurretState (Variables|Default|GetTurretState)
    (:NewEnumerator0
      (CallFunction|RotateTurret))
    (:NewEnumerator1
      (CallFunction|AttackTurret))))

(fn ConstructionScript)

(fn UpdateBeam
  (if (Variables|Default|GetIsBeamActive)
    (bind (_outhit _returnvalue) (Collision|LineTraceByChannel (Transformation|GetSocketLocation (Variables|Default|GetPoseableMesh) "bn_headbarrelend") (Variables|Default|GetTargetLocation) "TraceTypeQuery2" false 0 "None"))
    (if _returnvalue
      (Effects|Components|ParticleSystem|SetVectorParameter (Variables|Default|GetBeam) "User.Beam End" (.Location (Collision|BreakHitResult _outhit))))))